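; Behavior tree task that ends an accusation dialogue and brings up the game over screen.
; On AI execute it hides the dialogue widget on the player stand-in and calls EndDialouge on the NPC controller.
; It then adds a GameOver widget to the viewport, shows the mouse cursor, pauses the game and re-enables player input.
; The task never calls Finish Execute.
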(event EventReceiveExecuteAI
  (params (OwnerController :type AI%20Controller%20Object%20Reference) (ControlledPawn :type Pawn%20Object%20Reference))
  (bind _returnvalue (Game|GetPlayerController 0))
  (bind _asplayer_standin_bp (Utilities|Casting|CastToPlayerStandinBP (Game|GetPlayerCharacter 0)))
  (Widget|SetVisibility (Variables|/Game/Blueprints/PlayerStandinBP.PlayerStandinBP_C|GetDialougeInstance _asplayer_standin_bp) "Hidden")
  (bind _asnpccontroller (Utilities|Casting|CastToNPCController OwnerController))
  (Default|EndDialouge _asnpccontroller)
  (bind _returnvalue_2 (UserInterface|CreateWidget "/Game/Blueprints/UI/GameOver.GameOver_C" (Game|GetPlayerController 0)))
  (UserInterface|Viewport|AddtoViewport _returnvalue_2 0)
  (Variables|/Script/Engine.PlayerController|SetbShowMouseCursor _returnvalue true)
  (Game|SetGamePaused true)
  (Input|EnableInput (Game|GetPlayerCharacter 0) _returnvalue))