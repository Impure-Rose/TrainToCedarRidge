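; Borge is an actor that rides on the actor referenced by George, attached at that actor's BorgeHolder socket.
; On BeginPlay it casts George's root component to a MeshComponent and attaches its own root to the socket, snapping location and scale while keeping relative rotation.
; Tick and the construction script are empty, and alternative attach calls remain unconnected.
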(event EventBeginPlay
  (bind _asmesh_component (Utilities|Casting|CastToMeshComponent (Variables|/Script/Engine.Actor|GetRootComponent (Variables|Default|GetGeorge))))
  (Transformation|AttachComponentToComponent (Variables|Default|GetDefaultSceneRoot) _asmesh_component "BorgeHolder" "SnapToTarget" "KeepRelative" "SnapToTarget" true))

(event Collision|EventActorBeginOverlap
  (params (OtherActor :type Actor%20Object%20Reference)))

(event EventTick
  (params (DeltaSeconds :type Float%20%28single-precision%29)))

(fn ConstructionScript)