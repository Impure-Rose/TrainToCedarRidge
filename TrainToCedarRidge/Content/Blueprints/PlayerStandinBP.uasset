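; Player character for a clue-gathering puzzle game, handling movement, sprint, look and interaction.
; BeginPlay restores clues and paper state from the ActiveGame autosave, clamps camera pitch and creates HUD, dialogue and journal widgets.
; Pause toggles the journal, and Interact messages the current interactable actor.
; Minigame events open the picture puzzle widget, or hide the mesh and switch to a second camera placed at the plunger or combo lock.
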(event Custom|StartDialouge
  (params (CharacterInitatingConversation :type Text))
  (Variables|/Script/Engine.PlayerController|SetbShowMouseCursor (Game|GetPlayerController 0) true))

(event Custom|BeginPaperMiniGame
  (bind _returnvalue (UserInterface|CreateWidget "/Game/Blueprints/Mingames/PictureMiniGame.PictureMiniGame_C" 0 0))
  (UserInterface|Viewport|AddtoViewport _returnvalue 0)
  (Variables|/Script/Engine.PlayerController|SetbShowMouseCursor (Game|GetPlayerController 0) true))

(event Custom|Endpaperminigame
  (Widget|RemovefromParent (stale Custom|BeginPaperMiniGame _returnvalue))
  (Variables|/Script/Engine.PlayerController|SetbShowMouseCursor (Game|GetPlayerController 0) false))

(event Custom|InPlunger
  (bind _camera1 (Variables|Default|GetCamera1))
  (Variables|Default|Setinteracting true)
  (Variables|Default|SetCanRotate false)
  (Rendering|SetVisibility (Variables|Character|GetMesh) false false)
  (Components|Activation|SetActive (Variables|Default|GetCamera) false false)
  (Components|Activation|SetActive _camera1 true false)
  (bind _outactors (Actor|GetAllActorsOfClass "/Game/Blueprints/PlungerMiniGame.PlungerMiniGame_C"))
  (for _array_element _outactors
    (Transformation|SetWorldLocation _camera1 (Transformation|GetWorldLocation (Variables|/Game/Blueprints/PlungerMiniGame.PlungerMiniGame_C|GetScene _array_element)) false false)
    (Transformation|SetWorldRotation _camera1 (Math|Conversions|RotationFromXVector (Math|Vector|GetForwardVector (Variables|/Game/Blueprints/PlungerMiniGame.PlungerMiniGame_C|GetScene _array_element))) false false)))

(event Custom|OutPlunger
  (Variables|Default|SetCanWalk true)
  (Variables|Default|SetCanRotate true)
  (Variables|Default|Setinteracting false)
  (Rendering|SetVisibility (Variables|Character|GetMesh) true false)
  (Components|Activation|SetActive (Variables|Default|GetCamera) true false)
  (Components|Activation|SetActive (Variables|Default|GetCamera1) false false))

(event Custom|ComboLockIn
  (bind _camera1 (Variables|Default|GetCamera1))
  (Variables|Default|Setinteracting true)
  (Variables|Default|SetCanRotate false)
  (Rendering|SetVisibility (Variables|Character|GetMesh) false false)
  (Components|Activation|SetActive (Variables|Default|GetCamera) false false)
  (Components|Activation|SetActive _camera1 true false)
  (bind _outactors (Actor|GetAllActorsOfClass "/Game/Blueprints/ComboLock.ComboLock_C"))
  (for _array_element _outactors
    (Transformation|SetWorldLocation _camera1 (Transformation|GetWorldLocation (Variables|/Game/Blueprints/ComboLock.ComboLock_C|GetScene _array_element)) false false)
    (Transformation|SetWorldRotation _camera1 (Math|Conversions|RotationFromXVector (Math|Vector|GetForwardVector (Variables|/Game/Blueprints/ComboLock.ComboLock_C|GetScene _array_element))) false false)))

(event Custom|ComboLockOut
  (Variables|Default|SetCanWalk true)
  (Variables|Default|SetCanRotate true)
  (Variables|Default|Setinteracting false)
  (Rendering|SetVisibility (Variables|Character|GetMesh) true false)
  (Components|Activation|SetActive (Variables|Default|GetCamera) true false)
  (Components|Activation|SetActive (Variables|Default|GetCamera1) false false))

(event EventBeginPlay
  (bind _returnvalue (Game|GetPlayerCameraManager 0))
  (bind _returnvalue_2 (SaveGame|DoesSaveGameExist "ActiveGame"))
  (if _returnvalue_2
    (bind _savegame (|AsyncLoadGamefromSlot "ActiveGame")
      (:then
        (bind _asautosave (Utilities|Casting|CastToAutosave _savegame))
        (Variables|Default|SetSeenClues (Variables|/Game/Blueprints/Autosave.Autosave_C|GetClueInventory _asautosave))
        (Variables|Default|SetHasPaper (Variables|/Game/Blueprints/Autosave.Autosave_C|GetHasPaper _asautosave)))))
  (Variables|/Script/Engine.PlayerCameraManager|SetViewPitchMin _returnvalue -9e+01)
  (Variables|/Script/Engine.PlayerCameraManager|SetViewPitchMax _returnvalue 1e+01)
  (bind _returnvalue_3 (UserInterface|CreateWidget "/Game/Blueprints/UI/HUD.HUD_C" (Game|GetPlayerController 0)))
  (bind _output_get (Variables|Default|SetHUDInstance _returnvalue_3))
  (UserInterface|Viewport|AddtoViewport _output_get 0)
  (bind _returnvalue_4 (UserInterface|CreateWidget "/Game/Blueprints/UI/Dialouge.Dialouge_C" (Game|GetPlayerController 0)))
  (bind _output_get_2 (Variables|Default|SetDialougeInstance _returnvalue_4))
  (UserInterface|Viewport|AddtoViewport _output_get_2 0)
  (Widget|SetVisibility _returnvalue_4 "Hidden")
  (bind _returnvalue_5 (UserInterface|CreateWidget "/Game/Blueprints/UI/Journal.Journal_C" (Game|GetPlayerController 0)))
  (Variables|Default|SetJournal _returnvalue_5))

(event Collision|EventActorBeginOverlap
  (params (OtherActor :type Actor%20Object%20Reference)))

(event EventTick
  (params (DeltaSeconds :type Float%20%28single-precision%29)))

(event Input|ActionEvents|InputActionPause
  (params (Key :type Key%20Structure :default "None"))
  (bind _journal (Variables|Default|GetJournal))
  ;[1 1 1] Pause
  (:Pressed
    (if (Variables|Default|GetIsPaused)
      (Variables|Default|SetIsPaused false)
      (Widget|RemovefromParent _journal)
      (Game|SetGamePaused false)
      (Variables|/Script/Engine.PlayerController|SetbShowMouseCursor (Game|GetPlayerController 0) false)
      (else
        (Variables|Default|SetIsPaused true)
        (UserInterface|Viewport|AddtoViewport _journal 0)
        (Game|SetGamePaused true)
        (Variables|/Script/Engine.PlayerController|SetbShowMouseCursor (Game|GetPlayerController 0) true)))))

(event Input|ActionEvents|InputActionInteract
  (params (Key :type Key%20Structure :default "None"))
  (bind _interactableactor (Variables|Default|GetInteractableActor))
  (:Pressed
    (Utilities|IsValid _interactableactor
      (:Is%20Valid
        (if (not (Variables|Default|Getinteracting))
          (Class|InteractionBPI|Interact(Message) _interactableactor))))))

(event Input|AxisEvents|InputAxisMoveForward
  (params (AxisValue :type Float%20%28single-precision%29))
  ;[1 1 1] Movement Tools
  (if (Variables|Default|GetCanWalk)
    (Pawn|Input|AddMovementInput (Math|Vector|GetForwardVector (Math|Rotator|MakeRotator 0.0 0.0 (.Yaw (Math|Rotator|BreakRotator (Pawn|GetControlRotation :!class /Script/Engine.Pawn))))) AxisValue false)))

(event Input|AxisEvents|InputAxisMoveRight
  (params (AxisValue :type Float%20%28single-precision%29))
  ;[1 1 1] Movement Tools
  (if (Variables|Default|GetCanWalk)
    (Pawn|Input|AddMovementInput (Math|Vector|GetRightVector (Math|Rotator|MakeRotator 0.0 0.0 (.Yaw (Math|Rotator|BreakRotator (Pawn|GetControlRotation :!class /Script/Engine.Pawn))))) AxisValue false)))

(event Input|AxisEvents|InputAxisLookUp
  (params (AxisValue :type Float%20%28single-precision%29))
  ;[1 1 1] Movement Tools
  (if (Variables|Default|GetCanRotate)
    (Pawn|Input|AddControllerPitchInput AxisValue)))

(event Input|AxisEvents|InputAxisTurn
  (params (AxisValue :type Float%20%28single-precision%29))
  ;[1 1 1] Movement Tools
  (if (Variables|Default|GetCanRotate)
    (Pawn|Input|AddControllerYawInput AxisValue)))

(event Input|KeyboardEvents|E
  (params (Key :type Key%20Structure :default "None"))
  (:Pressed
    (if (Variables|Default|GetInUI)
      (Widget|RemovefromParent (Variables|Default|GetUIElementToDismiss)))))

(event Input|KeyboardEvents|LeftShift
  (params (Key :type Key%20Structure :default "None"))
  ;[1 1 1] Movement Tools
  (:Pressed
    (Variables|/Script/Engine.CharacterMovementComponent|SetMaxWalkSpeed (Variables|Character|GetCharacterMovement) 5e+02))
  (:Released
    (Variables|/Script/Engine.CharacterMovementComponent|SetMaxWalkSpeed (Variables|Character|GetCharacterMovement) 2.8e+02)))

(fn ConstructionScript)