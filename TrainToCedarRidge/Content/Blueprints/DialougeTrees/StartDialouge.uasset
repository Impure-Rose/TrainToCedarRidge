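; StartDialouge is a behavior tree task that opens dialogue between the AI and the player.
; It casts the player character to PlayerStandinBP, makes that character's dialogue widget visible and stores it in a Blackboard key, after printing a debug greeting.
; It then shows the mouse cursor, disables character input and finishes successfully.
; A failed cast stops execution without finishing the task.
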(event EventReceiveExecuteAI
  (params (OwnerController :type AI%20Controller%20Object%20Reference) (ControlledPawn :type Pawn%20Object%20Reference))
  (bind _returnvalue (Game|GetPlayerController 0))
  (Development|PrintString "Hello")
  (bind _asplayer_standin_bp (Utilities|Casting|CastToPlayerStandinBP (Game|GetPlayerCharacter 0)))
  (Widget|SetVisibility (Variables|/Game/Blueprints/PlayerStandinBP.PlayerStandinBP_C|GetDialougeInstance _asplayer_standin_bp) "SelfHitTestInvisible")
  (Class|BTFunctionLibrary|SetBlackboardValueasObject (Variables|Default|GetBB_DialougeUI) (Variables|/Game/Blueprints/PlayerStandinBP.PlayerStandinBP_C|GetDialougeInstance _asplayer_standin_bp))
  (Variables|/Script/Engine.PlayerController|SetbShowMouseCursor _returnvalue true)
  (Input|DisableInput (Game|GetPlayerCharacter 0) _returnvalue)
  (AI|BehaviorTree|FinishExecute true))