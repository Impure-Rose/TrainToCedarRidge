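; Behavior tree task for dialogue trees that asks a question and waits for the player to pick a response.
; On execute it gets the dialogue UI from the blackboard, sets its text and adds a bound, clickable widget for each response.
; Selection writes the chosen option to the blackboard as a string, clears the options and finishes the task successfully.
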(event Custom|ResponseSelection
  (params (SelectedOption :type Text))
  (Class|BTFunctionLibrary|SetBlackboardValueasString (Variables|Default|GetBB_Response) (Utilities|String|ToString(Text) SelectedOption))
  (Widget|Panel|ClearChildren (Variables|/Game/Blueprints/UI/Dialouge.Dialouge_C|GetOptionHolding (Variables|Default|GetDialougeUI)))
  (AI|BehaviorTree|FinishExecute true))

(event EventReceiveExecuteAI
  (params (OwnerController :type AI%20Controller%20Object%20Reference) (ControlledPawn :type Pawn%20Object%20Reference))
  (bind _asdialouge (Utilities|Casting|CastToDialouge (Class|BTFunctionLibrary|GetBlackboardValueasObject (Variables|Default|GetBB_DialougeUI))))
  (bind _output_get (Variables|Default|SetDialougeUI _asdialouge))
  (Variables|/Game/Blueprints/UI/Dialouge.Dialouge_C|SetWhatToSay _output_get (Variables|Default|GetText))
  (CallFunction|PrepareResponses))

(fn PrepareResponses
  (for _array_element (Variables|Default|GetResponses)
    (bind _returnvalue (UserInterface|CreateWidget "/Game/Blueprints/UI/Responses.Responses_C"))
    (Rendering|Components|TextRender|SetText (Variables|/Game/Blueprints/UI/Responses.Responses_C|GetResponseText _returnvalue) _array_element)
    (Class|VerticalBox|AddChildtoVerticalBox (Variables|/Game/Blueprints/UI/Dialouge.Dialouge_C|GetOptionHolding (Variables|Default|GetDialougeUI)) _returnvalue)
    (EventDispatchers|BindEventtoResponseClick _returnvalue (EventDispatchers|CreateEvent :!event Custom|ResponseSelection))))