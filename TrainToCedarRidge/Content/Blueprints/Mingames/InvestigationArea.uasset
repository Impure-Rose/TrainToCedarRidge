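; Investigation spot actor that lets the player open a picture minigame, which may hold a clue.
; It starts hidden and non-colliding until RNGActive enables its box collision and Niagara effect.
; Overlap toggles input and the HUD interact prompt, and Interact creates the PictureMiniGame widget with HasClue, shows the cursor and disables actor input.
; ClueFound turns off the collision and effect.
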(event EventBeginPlay
  (Collision|SetCollisionEnabled (Variables|Default|GetBox) "NoCollision")
  (Rendering|SetVisibility (Variables|Default|GetNiagara) false false))

(event EventRNGActive
  (Collision|SetCollisionEnabled (Variables|Default|GetBox) "QueryAndPhysics")
  (Rendering|SetVisibility (Variables|Default|GetNiagara) true false))

(event EventTick
  (params (DeltaSeconds :type Float%20%28single-precision%29)))

(event Collision|EventActorBeginOverlap
  (params (OtherActor :type Actor%20Object%20Reference))
  (Input|EnableInput (Game|GetPlayerController 0))
  (bind _asplayer_standin_bp (Utilities|Casting|CastToPlayerStandinBP (Game|GetPlayerCharacter 0)))
  (Widget|SetVisibility (Variables|/Game/Blueprints/UI/HUD.HUD_C|GetInteractPrompt (Variables|/Game/Blueprints/PlayerStandinBP.PlayerStandinBP_C|GetHUDInstance _asplayer_standin_bp)) "SelfHitTestInvisible"))

(event Collision|EventActorEndOverlap
  (params (OtherActor :type Actor%20Object%20Reference))
  (Input|DisableInput (Game|GetPlayerController 0))
  (bind _asplayer_standin_bp (Utilities|Casting|CastToPlayerStandinBP (Game|GetPlayerCharacter 0)))
  (Widget|SetVisibility (Variables|/Game/Blueprints/UI/HUD.HUD_C|GetInteractPrompt (Variables|/Game/Blueprints/PlayerStandinBP.PlayerStandinBP_C|GetHUDInstance _asplayer_standin_bp)) "Hidden"))

(event EventClueFound
  (bind _niagara (Variables|Default|GetNiagara))
  (Collision|SetCollisionEnabled (Variables|Default|GetBox) "NoCollision")
  (Class|NiagaraComponent|SetPaused _niagara true)
  (Rendering|SetVisibility _niagara false false))

(event Input|ActionEvents|InputActionInteract
  (params (Key :type Key%20Structure :default "None"))
  (bind _returnvalue (Game|GetPlayerController 0))
  (:Pressed
    (bind _returnvalue_2 (UserInterface|CreateWidget "/Game/Blueprints/Mingames/PictureMiniGame.PictureMiniGame_C" (Game|GetPlayerController 0) 0 (Variables|Default|Gethas%20Clue)))
    (UserInterface|Viewport|AddtoViewport _returnvalue_2 0)
    (Variables|/Script/Engine.PlayerController|SetbShowMouseCursor _returnvalue true)
    (Input|DisableInput _returnvalue)))

(fn ConstructionScript)