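; Behavior tree task that closes an NPC dialogue and returns control to the player.
; On execute it hides the dialogue widget held by PlayerStandinBP and calls EndDialouge on the owning NPCController.
; It then hides the mouse cursor, switches to game-only input and re-enables input on the player character.
; The task never calls Finish Execute, so it does not report completion to the tree itself.
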(event EventReceiveExecuteAI
  (params (OwnerController :type AI%20Controller%20Object%20Reference) (ControlledPawn :type Pawn%20Object%20Reference))
  (bind _returnvalue (Game|GetPlayerController 0))
  (bind _asplayer_standin_bp (Utilities|Casting|CastToPlayerStandinBP (Game|GetPlayerCharacter 0)))
  (Widget|SetVisibility (Variables|/Game/Blueprints/PlayerStandinBP.PlayerStandinBP_C|GetDialougeInstance _asplayer_standin_bp) "Hidden")
  (bind _asnpccontroller (Utilities|Casting|CastToNPCController OwnerController))
  (Default|EndDialouge _asnpccontroller)
  (Variables|/Script/Engine.PlayerController|SetbShowMouseCursor _returnvalue false)
  (Input|SetInputModeGameOnly _returnvalue)
  (Input|EnableInput (Game|GetPlayerCharacter 0) _returnvalue))