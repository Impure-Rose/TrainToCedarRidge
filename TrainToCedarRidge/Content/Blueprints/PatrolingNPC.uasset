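; Patrolling NPC actor that moves along the spline of a PatrolSpline actor found in the level at BeginPlay.
; A timeline, with play rate set from SecToComplete, maps its track to a distance along the spline and sets the actor's transform each update.
; Location and rotation are read in the spline's local space, with rotation always sampled at the spline start rather than the current distance.
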(event Custom|Move%20Object
  (bind _splineref (Variables|Default|GetSplineREF))
  (bind _spline (Variables|/Game/Blueprints/PatrolSpline.PatrolSpline_C|GetSpline _splineref))
  (Components|Timeline|SetPlayRate (Variables|Default|GetMove%20Obj%20Timeline) (/ 1.0 (Variables|Default|GetSecToComplete)))
  (bind _movetrack (Timeline|Move%20Obj%20Timeline Play)
    (:Update
      (Transformation|SetActorTransform (Math|Transform|MakeTransform (Spline|GetLocationatDistanceAlongSpline _spline (Math|Float|Lerp 0.0 (Spline|GetSplineLength (Variables|/Game/Blueprints/PatrolSpline.PatrolSpline_C|GetSpline (Variables|Default|GetSplineREF))) _movetrack) "Local") (Spline|GetRotationatDistanceAlongSpline _spline 0.0 "Local") "1,1,1")))))

(event EventBeginPlay
  (bind _returnvalue (Actor|GetActorOfClass "/Game/Blueprints/PatrolSpline.PatrolSpline_C"))
  (Variables|Default|SetSplineREF _returnvalue)
  (CallFunction|MoveObject))

(event Collision|EventActorBeginOverlap
  (params (OtherActor :type Actor%20Object%20Reference)))

(event EventTick
  (params (DeltaSeconds :type Float%20%28single-precision%29)))

(fn ConstructionScript)