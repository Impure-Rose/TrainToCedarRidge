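; ToolRack is an interactable actor that shows a scissors notification and plants a clue in a random investigation area.
; Overlap enables input and shows the HUD interact prompt; leaving reverses both.
; Interact displays the ScissorsNotify widget for two seconds behind a multi-input do-once gate, then resets it.
; The first reset also flags a random InvestigationArea from Targets as holding the clue and sends RNGActiveMessage to Targets.
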(event EventBeginPlay)

(event EventTick
  (params (DeltaSeconds :type Float%20%28single-precision%29)))

(event Collision|EventActorBeginOverlap
  (params (OtherActor :type Actor%20Object%20Reference))
  (Input|EnableInput (Game|GetPlayerController 0))
  (bind _asplayer_standin_bp (Utilities|Casting|CastToPlayerStandinBP (Game|GetPlayerCharacter 0)))
  (Widget|SetVisibility (Variables|/Game/Blueprints/UI/HUD.HUD_C|GetInteractPrompt (Variables|/Game/Blueprints/PlayerStandinBP.PlayerStandinBP_C|GetHUDInstance _asplayer_standin_bp)) "SelfHitTestInvisible"))

(event Collision|EventActorEndOverlap
  (params (OtherActor :type Actor%20Object%20Reference))
  (Input|DisableInput (Game|GetPlayerController 0))
  (bind _asplayer_standin_bp (Utilities|Casting|CastToPlayerStandinBP (Game|GetPlayerCharacter 0)))
  (Widget|SetVisibility (Variables|/Game/Blueprints/UI/HUD.HUD_C|GetInteractPrompt (Variables|/Game/Blueprints/PlayerStandinBP.PlayerStandinBP_C|GetHUDInstance _asplayer_standin_bp)) "Hidden"))

(event Input|ActionEvents|InputActionInteract
  (params (Key :type Key%20Structure))
  (:Pressed
    (|DoOnceMultiInput :!label _label
      (:A%20Out
        (bind _returnvalue (UserInterface|CreateWidget "/Game/Blueprints/Mingames/ScissorsNotify.ScissorsNotify_C" (Game|GetPlayerController 0)))
        (UserInterface|Viewport|AddtoViewport _returnvalue 0)
        (Utilities|FlowControl|Delay 2.0)
        (Widget|RemovefromParent _returnvalue)
        (goto _label Reset%20In))
      (:Reset%20Out
        (Utilities|FlowControl|DoOnce false
          (:Completed
            (bind _asinvestigation_area (Utilities|Casting|CastToInvestigationArea (.OutItem (Utilities|Array|Random (Variables|Default|GetTargets)))))
            (Variables|/Game/Blueprints/Mingames/InvestigationArea.InvestigationArea_C|Sethas%20Clue _asinvestigation_area true)
            (Class|ScissorHuntBPI|RNGActive(Message) (Variables|Default|GetTargets))))))))

(fn ConstructionScript)