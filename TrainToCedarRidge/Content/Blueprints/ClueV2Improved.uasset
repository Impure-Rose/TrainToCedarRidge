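; ClueV2Improved is a configurable clue pickup that the player inspects once with the Interact key.
; Overlap enables input and shows the player HUD's interact prompt; leaving reverses both.
; Interacting records the clue in PlayerStandinBP's SeenClues, opens a PlungerFoundClue widget as the dismissible UI, then destroys the actor.
; The construction script applies the mesh and collision box size when a mesh is set.
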(event EventBeginPlay)

(event EventTick
  (params (DeltaSeconds :type Float%20%28single-precision%29)))

(event Collision|EventActorBeginOverlap
  (params (OtherActor :type Actor%20Object%20Reference))
  (Input|EnableInput (Game|GetPlayerController 0))
  (bind _asplayer_standin_bp (Utilities|Casting|CastToPlayerStandinBP (Game|GetPlayerCharacter 0)))
  (Widget|SetVisibility (Variables|/Game/Blueprints/UI/HUD.HUD_C|GetInteractPrompt (Variables|/Game/Blueprints/PlayerStandinBP.PlayerStandinBP_C|GetHUDInstance _asplayer_standin_bp)) "SelfHitTestInvisible"))

(event Collision|EventActorEndOverlap
  (params (OtherActor :type Actor%20Object%20Reference))
  (Input|DisableInput (Game|GetPlayerController 0))
  (bind _asplayer_standin_bp (Utilities|Casting|CastToPlayerStandinBP (Game|GetPlayerCharacter 0)))
  (Widget|SetVisibility (Variables|/Game/Blueprints/UI/HUD.HUD_C|GetInteractPrompt (Variables|/Game/Blueprints/PlayerStandinBP.PlayerStandinBP_C|GetHUDInstance _asplayer_standin_bp)) "Hidden"))

(event Input|ActionEvents|InputActionInteract
  (params (Key :type Key%20Structure :default "None"))
  (:Pressed
    (if (not (Variables|Debug|GetSeenBefore))
      (Variables|Debug|SetSeenBefore true)
      (bind _asplayer_standin_bp (Utilities|Casting|CastToPlayerStandinBP (Game|GetPlayerCharacter 0)))
      (Utilities|Map|Add (Variables|/Game/Blueprints/PlayerStandinBP.PlayerStandinBP_C|GetSeenClues _asplayer_standin_bp) (Variables|ForInventorySystem|GetClueToSee) true)
      (bind _returnvalue (UserInterface|CreateWidget "/Game/Blueprints/UI/plungerFoundClue.plungerFoundClue_C" (Game|GetPlayerController 0) (Variables|ClueFoundUI|GetImage) (Variables|ClueFoundUI|GetDescription%20Text)))
      (bind _asplayer_standin_bp_2 (Utilities|Casting|CastToPlayerStandinBP (Game|GetPlayerCharacter 0)))
      (Variables|/Game/Blueprints/PlayerStandinBP.PlayerStandinBP_C|SetInUI _asplayer_standin_bp_2 true)
      (Variables|/Game/Blueprints/PlayerStandinBP.PlayerStandinBP_C|SetUIElementToDismiss _asplayer_standin_bp_2 _returnvalue)
      (UserInterface|Viewport|AddtoViewport _returnvalue 0)
      (Actor|DestroyActor))))

(fn ConstructionScript
  (Utilities|IsValid (Variables|VisualElements|GetClueMesh)
    (:Is%20Valid
      (Components|StaticMesh|SetStaticMesh (Variables|Default|GetCluePlaceholder) (Variables|VisualElements|GetClueMesh))
      (Components|Box|SetBoxExtent (Variables|Default|GetBox) (Variables|Collisions|GetCollisionSize) true))))