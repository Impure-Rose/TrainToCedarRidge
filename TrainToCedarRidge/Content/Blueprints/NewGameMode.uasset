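; Game mode that randomly casts a killer and a victim from a Suspects list for what appears to be a murder mystery.
; On BeginPlay, when no save exists under the blank slot name, it picks and prints the Killer.
; A re-roll loop aims at a different Victim, but its comparison draws a separate random suspect, so the two can still match.
; Nothing is saved; Tick and construction are empty.
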(event EventBeginPlay
  (bind _suspects (Variables|Default|GetSuspects))
  (bind _outitem (Utilities|Array|Random _suspects))
  ;[1 1 1] Generate Killers
  (bind _returnvalue (SaveGame|DoesSaveGameExist))
  (if (not _returnvalue)
    (bind _output_get (Variables|Default|SetKiller (.OutItem (Utilities|Array|Random (Variables|Default|GetSuspects)))))
    (Development|PrintString _output_get)
    (while (Utilities|Enum|Equal(Enum) _output_get _outitem)
      (Variables|Default|SetVictim _outitem)
      (Development|PrintString (Variables|Default|GetVictim)))
    (Development|PrintString (Variables|Default|GetVictim))))

(event EventTick
  (params (DeltaSeconds :type Float%20%28single-precision%29)))

(fn ConstructionScript)