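; NPCV2 is an interactable NPC that starts dialogue through its NPCController.
; Actor overlaps set or clear it as the PlayerStandinBP's interactable and toggle the HUD prompt, without checking which actor overlapped.
; BeginPlay copies DialougeTree to the controller before selecting the intro or general tree from HaveSpokenTo.
; Interact sets that flag and calls StartDialouge, without reselecting the tree.
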(event EventBeginPlay
  (bind _asnpccontroller (Utilities|Casting|CastToNPCController (AI|GetAIController self)))
  (Variables|/Game/Blueprints/NPCController.NPCController_C|SetDialougeTree _asnpccontroller (Variables|DialougeTreeToUse|GetDialougeTree))
  (if (Variables|Default|GetHaveSpokenTo)
    (Variables|DialougeTreeToUse|SetDialougeTree (Variables|DialougeTreeToUse|GetGenTree))
    (else
      (Variables|DialougeTreeToUse|SetDialougeTree (Variables|DialougeTreetoUse|GetIntroTree)))))

(event EventTick
  (params (DeltaSeconds :type Float%20%28single-precision%29)))

(event Collision|EventActorBeginOverlap
  (params (OtherActor :type Actor%20Object%20Reference))
  ;[1 1 1] Show or remove notice of interaction
  (bind _asplayer_standin_bp (Utilities|Casting|CastToPlayerStandinBP (Game|GetPlayerCharacter 0)))
  (Variables|/Game/Blueprints/PlayerStandinBP.PlayerStandinBP_C|Setinteractable _asplayer_standin_bp true)
  (Variables|/Game/Blueprints/PlayerStandinBP.PlayerStandinBP_C|SetInteractableActor _asplayer_standin_bp self)
  (Widget|SetVisibility (Variables|/Game/Blueprints/UI/HUD.HUD_C|GetInteractPrompt (Variables|/Game/Blueprints/PlayerStandinBP.PlayerStandinBP_C|GetHUDInstance _asplayer_standin_bp)) "SelfHitTestInvisible"))

(event Collision|EventActorEndOverlap
  (params (OtherActor :type Actor%20Object%20Reference))
  ;[1 1 1] Show or remove notice of interaction
  (bind _asplayer_standin_bp (Utilities|Casting|CastToPlayerStandinBP (Game|GetPlayerCharacter 0)))
  (Variables|/Game/Blueprints/PlayerStandinBP.PlayerStandinBP_C|Setinteractable _asplayer_standin_bp false)
  (Variables|/Game/Blueprints/PlayerStandinBP.PlayerStandinBP_C|SetInteractableActor _asplayer_standin_bp 0)
  (Widget|SetVisibility (Variables|/Game/Blueprints/UI/HUD.HUD_C|GetInteractPrompt (Variables|/Game/Blueprints/PlayerStandinBP.PlayerStandinBP_C|GetHUDInstance _asplayer_standin_bp)) "Hidden"))

(event EventInteract
  (Development|PrintString "anyone home")
  (Variables|Default|SetHaveSpokenTo true)
  (bind _asnpccontroller (Utilities|Casting|CastToNPCController (AI|GetAIController self)))
  (Default|StartDialouge _asnpccontroller))

(fn ConstructionScript)