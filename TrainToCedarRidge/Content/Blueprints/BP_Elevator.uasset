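; BP_Elevator is a two-floor elevator that moves its car between bottom and top via timelines lerping relative location.
; Door triggers on each floor call the car from the opposite end and open doors by shrinking their scale, reversing after a delay.
; The Elevator_Bottom trigger accepts only PlayerStandinBP, then after a delay alternates up and down trips by FlipFlop rather than car position.
; Position-checking branches for trips remain unwired.
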(event OnComponentBeginOverlap(Doors_Bottom)
  (params (OverlappedComponent :type Primitive%20Component%20Object%20Reference) (OtherActor :type Actor%20Object%20Reference) (OtherComp :type Primitive%20Component%20Object%20Reference) (OtherBodyIndex :type Integer) (bFromSweep :type Boolean) (SweepResult :type Hit%20Result%20Structure%20%28by%20ref%29))
  (if (== (.z (Variables|/Script/Engine.SceneComponent|GetRelativeLocation (Variables|Default|GetElevatorCar))) 454.0)
    (bind _newtrack_0 (Timeline|Timeline_2 Play)
      (:Update
        (Transformation|SetRelativeLocation (Variables|Default|GetElevatorCar) (Math|Vector|Lerp(Vector) "0, 0,454.000000" "0, 0, 0" _newtrack_0) false false)
        (bind _newtrack_0_2 (Timeline|Doors PlayFromStart)
          (:Update
            (Transformation|SetRelativeScale3D (Variables|Default|GetDoor_Left) (Math|Vector|Lerp(Vector) "1.000000,1.000000,1.330421" "1.000000,0.500000,1.330421" _newtrack_0_2))
            (Utilities|FlowControl|Delay 5.0)
            (Timeline|Doors ReverseFromEnd)))))
    (else
      (Timeline|Doors PlayFromStart))))

(event OnComponentBeginOverlap(Doors_Top)
  (params (OverlappedComponent :type Primitive%20Component%20Object%20Reference) (OtherActor :type Actor%20Object%20Reference) (OtherComp :type Primitive%20Component%20Object%20Reference) (OtherBodyIndex :type Integer) (bFromSweep :type Boolean) (SweepResult :type Hit%20Result%20Structure%20%28by%20ref%29))
  (if (== (.z (Variables|/Script/Engine.SceneComponent|GetRelativeLocation (Variables|Default|GetElevatorCar))) 0.0)
    (bind _newtrack_0 (Timeline|Timeline_3 Play)
      (:Update
        (Transformation|SetRelativeLocation (Variables|Default|GetElevatorCar) (Math|Vector|Lerp(Vector) "0, 0, 0" "0.000000,0.000000,454.000000" _newtrack_0) false false)
        (bind _newtrack_0_2 (Timeline|Timeline_1 PlayFromStart)
          (:Update
            (Transformation|SetRelativeScale3D (Variables|Default|GetDoor_Right1) (Math|Vector|Lerp(Vector) "1.000000,1.000000,1.330421" "1.000000,0.500000,1.330421" _newtrack_0_2))
            (Utilities|FlowControl|Delay 5.0)
            (Timeline|Timeline_1 ReverseFromEnd)))))
    (else
      (Timeline|Timeline_1 PlayFromStart))))

(event OnComponentBeginOverlap(Elevator_Bottom)
  (params (OverlappedComponent :type Primitive%20Component%20Object%20Reference) (OtherActor :type Actor%20Object%20Reference) (OtherComp :type Primitive%20Component%20Object%20Reference) (OtherBodyIndex :type Integer) (bFromSweep :type Boolean) (SweepResult :type Hit%20Result%20Structure%20%28by%20ref%29))
  (Utilities|Casting|CastToPlayerStandinBP OtherActor)
  (Utilities|FlowControl|FlipFlop
    (:A
      (Utilities|FlowControl|Delay 2.0)
      (bind _newtrack_0 (Timeline|Timeline_0 PlayFromStart)
        (:Update
          (Transformation|SetRelativeLocation (Variables|Default|GetElevatorCar) (Math|Vector|Lerp(Vector) "0, 0, 0" "0.000000,0.000000,454.000000" _newtrack_0) false false))))
    (:B
      (Utilities|FlowControl|Delay 2.0)
      (bind _newtrack_0_2 (Timeline|Timeline_4 PlayFromStart)
        (:Update
          (Transformation|SetRelativeLocation (Variables|Default|GetElevatorCar) (Math|Vector|Lerp(Vector) "0, 0,454.000000" "0, 0, 0" _newtrack_0_2) false false))))))

(event EventBeginPlay)

(event Collision|EventActorBeginOverlap
  (params (OtherActor :type Actor%20Object%20Reference)))

(event EventTick
  (params (DeltaSeconds :type Float%20%28single-precision%29)))

(fn ConstructionScript)