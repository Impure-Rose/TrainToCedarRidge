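; BP_InteractableDoor_Drawer is a configurable door or drawer that opens by itself three seconds after BeginPlay, with no interaction logic in the graph.
; Swings selects between two timelines: one yaws GeneralMesh to OpenAngle, the other slides it along Y to NewLocationY.
; The construction script applies mesh and scale, offsets Sphere to NewLocationY, and either sets up the interior ObjectToSee mesh or destroys it, depending on HasItem.
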(event EventBeginPlay
  (Utilities|FlowControl|Delay 3.0)
  (if (Variables|Default|GetSwings)
    ;[1 1 1] Opening Pull
    (bind _timer (Timeline|Swing PlayFromStart)
      (:Update
        (Transformation|SetRelativeRotation (Variables|Default|GetGeneralMesh) (Math|Rotator|MakeRotator 0.0 0.0 (Math|Float|Lerp 0.0 (Variables|Default|GetOpenAngle) _timer)) false false)))
    (else
      ;[1 1 1] Pull Out
      (bind _newtrack_0 (Timeline|Pulls PlayFromStart)
        (:Update
          (Transformation|SetRelativeLocation (Variables|Default|GetGeneralMesh) (Math|Vector|MakeVector 0.0 (Math|Float|Lerp 0.0 (Variables|Default|GetNew%20Location%20Y) _newtrack_0) 0.0) false false))))))

(fn ConstructionScript
  (bind _generalmesh (Variables|Default|GetGeneralMesh))
  (bind _objecttosee (Variables|Default|GetObjectToSee))
  (Components|StaticMesh|SetStaticMesh _generalmesh (Variables|Default|GetNew%20Mesh))
  (Transformation|SetRelativeScale3D _generalmesh (Variables|Default|GetSize))
  (Transformation|SetRelativeLocation (Variables|Default|GetSphere) (Math|Vector|MakeVector 0.0 (Variables|Default|GetNew%20Location%20Y) 0.0) false false)
  (if (Variables|Default|GetHas%20Item)
    (Components|StaticMesh|SetStaticMesh _objecttosee (Variables|Default|GetInterior%20Mesh))
    (Transformation|SetRelativeScale3D _objecttosee (Variables|Default|GetInteriorScale))
    (else
      (Components|DestroyComponent _objecttosee))))