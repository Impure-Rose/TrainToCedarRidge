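; AI controller for an NPC that starts and ends dialogue driven by a behavior tree.
; StartDialouge prints and runs the DialougeTree behavior tree, then hides the meshes of the player's PlayerStandinBP and the controlled NPCV2 pawn, including child components.
; EndDialouge stops the brain component's logic and makes both meshes visible again.
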(event Custom|StartDialouge
  (bind _dialougetree (Variables|Default|GetDialougeTree))
  (Development|PrintString (Utilities|GetDisplayName _dialougetree))
  (AI|RunBehaviorTree _dialougetree)
  (bind _asplayer_standin_bp (Utilities|Casting|CastToPlayerStandinBP (Game|GetPlayerCharacter 0)))
  (Rendering|SetVisibility (Variables|/Script/Engine.Character|GetMesh _asplayer_standin_bp) false true)
  (bind _asnpcv2 (Utilities|Casting|CastToNPCV2 (Pawn|GetControlledPawn)))
  (Rendering|SetVisibility (Variables|/Script/Engine.Character|GetMesh _asnpcv2) false true))

(event Custom|EndDialouge
  (AI|Logic|StopLogic (Variables|Default|GetBrainComponent) "")
  (bind _asplayer_standin_bp (Utilities|Casting|CastToPlayerStandinBP (Game|GetPlayerCharacter 0)))
  (Rendering|SetVisibility (Variables|/Script/Engine.Character|GetMesh _asplayer_standin_bp) true true)
  (bind _asnpcv2 (Utilities|Casting|CastToNPCV2 (Pawn|GetControlledPawn)))
  (Rendering|SetVisibility (Variables|/Script/Engine.Character|GetMesh _asnpcv2) true true))

(event EventBeginPlay)

(event EventTick
  (params (DeltaSeconds :type Float%20%28single-precision%29)))

(fn ConstructionScript)