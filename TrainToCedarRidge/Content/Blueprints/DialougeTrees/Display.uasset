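; Behavior Tree task that shows one line of NPC dialogue and waits for the player to advance it.
; On execute it feeds its Text, plus the NPCV2 pawn's name and portrait, to the Dialouge widget stored in the Blackboard.
; Tick gates on E or left mouse, then checks the Interact mappings.
; A matching press raises CharsPerSecond if still writing, clears the text and finishes successfully.
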(event EventReceiveExecuteAI
  (params (OwnerController :type AI%20Controller%20Object%20Reference) (ControlledPawn :type Pawn%20Object%20Reference))
  (bind _asdialouge (Utilities|Casting|CastToDialouge (Class|BTFunctionLibrary|GetBlackboardValueasObject (Variables|Default|GetDialougeWidget))))
  (Variables|/Game/Blueprints/UI/Dialouge.Dialouge_C|SetWhatToSay _asdialouge (Variables|Default|GetText))
  (Default|Write _asdialouge)
  (bind _asnpcv2 (Utilities|Casting|CastToNPCV2 ControlledPawn))
  (Variables|/Game/Blueprints/UI/Dialouge.Dialouge_C|SetWhoIsTalking _asdialouge (Variables|/Game/Blueprints/NPCV2.NPCV2_C|GetCharacterName _asnpcv2))
  (Class|Image|SetBrush (Variables|/Game/Blueprints/UI/Dialouge.Dialouge_C|GetImage_0 _asdialouge) (Utilities|Struct|MakeSlateBrush "(X=32.000000,Y=32.000000)" "(Left=0.000000,Top=0.000000,Right=0.000000,Bottom=0.000000)" "(SpecifiedColor=(R=1.000000,G=1.000000,B=1.000000,A=1.000000),ColorUseRule=UseColor_Specified)" (Variables|/Game/Blueprints/NPCV2.NPCV2_C|GetPortrait _asnpcv2) "Image" "NoTile" "NoMirror")))

(event EventTick
  (params (OwnerActor :type Actor%20Object%20Reference) (DeltaSeconds :type Float%20%28single-precision%29))
  (if (Game|Player|WasInputKeyJustPressed (Game|GetPlayerController 0) "E")
    (for _array_element (Class|InputSettings|GetActionMappingbyName (Class|InputSettings|GetInputSettings) "Interact") :!label _label
      (if (Game|Player|WasInputKeyJustPressed (Game|GetPlayerController 0) (.Key (Utilities|Struct|BreakInputActionKeyMapping _array_element)))
        (bind _asdialouge (Utilities|Casting|CastToDialouge (Class|BTFunctionLibrary|GetBlackboardValueasObject (Variables|Default|GetDialougeWidget))))
        (if (Variables|/Game/Blueprints/UI/Dialouge.Dialouge_C|GetWriting _asdialouge)
          (Variables|Default|SetCharsPerSecond 2e+02))
        (Variables|/Game/Blueprints/UI/Dialouge.Dialouge_C|SetWhatToSay _asdialouge "")
        (Default|Write _asdialouge)
        (AI|BehaviorTree|FinishExecute true)))
    (elif (Game|Player|WasInputKeyJustPressed (Game|GetPlayerController 0) "LeftMouseButton")
      (goto _label))))