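; Deprecated NPC actor (going by its file name) that lets the player start dialogue through the Interact input.
; Actor overlap events toggle input and the player HUD's interact prompt, without checking which actor overlapped.
; Interact passes the NPC's Name to PlayerStandinBP's StartDialouge, sets IsTalking and disables input, which Tick re-enables while the player is inside Sphere and not talking.
; The construction script applies NewMesh when valid.
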(event EventBeginPlay)

(event EventTick
  (params (DeltaSeconds :type Float%20%28single-precision%29))
  (if (Collision|IsOverlappingActor (Variables|Default|GetSphere) (Game|GetPlayerCharacter 0) :!class /Script/Engine.PrimitiveComponent)
    (bind _asplayer_standin_bp (Utilities|Casting|CastToPlayerStandinBP (Game|GetPlayerCharacter 0)))
    (if (not (Variables|/Game/Blueprints/PlayerStandinBP.PlayerStandinBP_C|GetIsTalking _asplayer_standin_bp))
      (Input|EnableInput (Game|GetPlayerController 0)))))

(event Collision|EventActorBeginOverlap
  (params (OtherActor :type Actor%20Object%20Reference))
  ;[1 1 1] Show or remove notice of interaction
  (Input|EnableInput (Game|GetPlayerController 0))
  (bind _asplayer_standin_bp (Utilities|Casting|CastToPlayerStandinBP (Game|GetPlayerCharacter 0)))
  (Widget|SetVisibility (Variables|/Game/Blueprints/UI/HUD.HUD_C|GetInteractPrompt (Variables|/Game/Blueprints/PlayerStandinBP.PlayerStandinBP_C|GetHUDInstance _asplayer_standin_bp)) "SelfHitTestInvisible"))

(event Collision|EventActorEndOverlap
  (params (OtherActor :type Actor%20Object%20Reference))
  ;[1 1 1] Show or remove notice of interaction
  (Input|DisableInput (Game|GetPlayerController 0))
  (bind _asplayer_standin_bp (Utilities|Casting|CastToPlayerStandinBP (Game|GetPlayerCharacter 0)))
  (Widget|SetVisibility (Variables|/Game/Blueprints/UI/HUD.HUD_C|GetInteractPrompt (Variables|/Game/Blueprints/PlayerStandinBP.PlayerStandinBP_C|GetHUDInstance _asplayer_standin_bp)) "Hidden"))

(event Input|ActionEvents|InputActionInteract
  (params (Key :type Key%20Structure :default "None"))
  ;[1 1 1] Start Dialouge
  (:Pressed
    (bind _asplayer_standin_bp (Utilities|Casting|CastToPlayerStandinBP (Game|GetPlayerCharacter 0)))
    (Default|StartDialouge _asplayer_standin_bp (Variables|Default|GetName))
    (Variables|/Game/Blueprints/PlayerStandinBP.PlayerStandinBP_C|SetIsTalking _asplayer_standin_bp true)
    (Input|DisableInput (Game|GetPlayerController 0))))

(fn ConstructionScript
  (bind _newmesh (Variables|Default|GetNewMesh))
  (if (Utilities|IsValid _newmesh)
    (Variables|Default|SetSkeletalMesh _newmesh)))