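; Sliding door actor that the player toggles with the Interact input while in its overlap area.
; Overlap begin and end enable or disable input for player 0 and show or hide the interact prompt on the PlayerStandinBP HUD, without checking which actor overlapped.
; A FlipFlop alternates two timelines, each adding a Y offset scaled by DoorTravel to the Door every update, so movement accumulates rather than interpolating between fixed positions.
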(event EventBeginPlay)

(event EventTick
  (params (DeltaSeconds :type Float%20%28single-precision%29)))

(event Collision|EventActorBeginOverlap
  (params (OtherActor :type Actor%20Object%20Reference))
  (Input|EnableInput (Game|GetPlayerController 0))
  (bind _asplayer_standin_bp (Utilities|Casting|CastToPlayerStandinBP (Game|GetPlayerCharacter 0)))
  (Widget|SetVisibility (Variables|/Game/Blueprints/UI/HUD.HUD_C|GetInteractPrompt (Variables|/Game/Blueprints/PlayerStandinBP.PlayerStandinBP_C|GetHUDInstance _asplayer_standin_bp)) "SelfHitTestInvisible"))

(event Collision|EventActorEndOverlap
  (params (OtherActor :type Actor%20Object%20Reference))
  (Input|DisableInput (Game|GetPlayerController 0))
  (bind _asplayer_standin_bp (Utilities|Casting|CastToPlayerStandinBP (Game|GetPlayerCharacter 0)))
  (Widget|SetVisibility (Variables|/Game/Blueprints/UI/HUD.HUD_C|GetInteractPrompt (Variables|/Game/Blueprints/PlayerStandinBP.PlayerStandinBP_C|GetHUDInstance _asplayer_standin_bp)) "Hidden"))

(event Input|ActionEvents|InputActionInteract
  (params (Key :type Key%20Structure :default "None"))
  (:Pressed
    (Utilities|FlowControl|FlipFlop
      (:A
        (bind _newtrack_0 (Timeline|Timeline_0 PlayFromStart)
          (:Update
            (Transformation|AddRelativeLocation (Variables|Default|GetDoor) (Math|Vector|MakeVector 0.0 (* _newtrack_0 (Variables|Default|GetDoorTravel)) 0.0) false false))))
      (:B
        (bind _newtrack_0_2 (Timeline|Timeline_1 PlayFromStart)
          (:Update
            (Transformation|AddRelativeLocation (Variables|Default|GetDoor) (Math|Vector|MakeVector 0.0 (* _newtrack_0_2 (Variables|Default|GetDoorTravel)) 0.0) false false)))))))

(fn ConstructionScript)