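; Behavior tree task for dialogue trees that lets the player choose a clue to present, or leave.
; On execute it takes the Dialouge widget from the blackboard and builds a Responses button for each player SeenClues entry flagged true, plus a Leave option.
; Response selection writes the chosen option to the blackboard as a string, clears the option list and finishes the task successfully.
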(event Custom|ResponseSelection
  (params (SelectedOption :type Text))
  (Class|BTFunctionLibrary|SetBlackboardValueasString (Variables|Default|GetBB_Response) (Utilities|String|ToString(Text) SelectedOption))
  (Widget|Panel|ClearChildren (Variables|/Game/Blueprints/UI/Dialouge.Dialouge_C|GetOptionHolding (Variables|Default|GetDialougeUI)))
  (AI|BehaviorTree|FinishExecute true))

(event EventReceiveExecuteAI
  (params (OwnerController :type AI%20Controller%20Object%20Reference) (ControlledPawn :type Pawn%20Object%20Reference))
  (bind _asdialouge (Utilities|Casting|CastToDialouge (Class|BTFunctionLibrary|GetBlackboardValueasObject (Variables|Default|GetBB_DialougeUI))))
  (Variables|Default|SetDialougeUI _asdialouge)
  (CallFunction|PrepareResponses))

(fn PrepareResponses
  (bind _dialougeui (Variables|Default|GetDialougeUI))
  (bind _optionholding (Variables|/Game/Blueprints/UI/Dialouge.Dialouge_C|GetOptionHolding _dialougeui))
  (bind _asplayer_standin_bp (Utilities|Casting|CastToPlayerStandinBP (Game|GetPlayerCharacter 0)))
  (bind _keys (Utilities|Map|Keys (Variables|/Game/Blueprints/PlayerStandinBP.PlayerStandinBP_C|GetSeenClues _asplayer_standin_bp)))
  (for _array_element _keys
    (bind _returnvalue (UserInterface|CreateWidget "/Game/Blueprints/UI/Responses.Responses_C"))
    (Rendering|Components|TextRender|SetText (Variables|/Game/Blueprints/UI/Responses.Responses_C|GetResponseText _returnvalue) (Utilities|Text|ToText(String) _array_element))
    (if (.Value (Utilities|Map|Find (Variables|/Game/Blueprints/PlayerStandinBP.PlayerStandinBP_C|GetSeenClues _asplayer_standin_bp) _array_element))
      (Class|VerticalBox|AddChildtoVerticalBox _optionholding _returnvalue)
      (EventDispatchers|BindEventtoResponseClick _returnvalue (EventDispatchers|CreateEvent :!event Custom|ResponseSelection))))
  (bind _returnvalue_2 (UserInterface|CreateWidget "/Game/Blueprints/UI/Responses.Responses_C"))
  (Rendering|Components|TextRender|SetText (Variables|/Game/Blueprints/UI/Responses.Responses_C|GetResponseText _returnvalue_2) "Leave")
  (Class|VerticalBox|AddChildtoVerticalBox _optionholding _returnvalue_2)
  (EventDispatchers|BindEventtoResponseClick _returnvalue_2 (EventDispatchers|CreateEvent :!event Custom|ResponseSelection)))