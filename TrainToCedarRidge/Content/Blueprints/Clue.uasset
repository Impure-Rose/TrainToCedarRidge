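; Clue is a placeable pickup actor that gives the player a paper.
; The construction script applies a per-instance mesh and, when that mesh is valid, the box collision size.
; Overlaps toggle the actor's input and the interact prompt on the PlayerStandinBP HUD, without checking which actor overlapped.
; Pressing Interact works once, setting HasPaper on the player and destroying the clue.
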(event EventBeginPlay)

(event EventTick
  (params (DeltaSeconds :type Float%20%28single-precision%29)))

(event Collision|EventActorBeginOverlap
  (params (OtherActor :type Actor%20Object%20Reference))
  (Input|EnableInput (Game|GetPlayerController 0))
  (bind _asplayer_standin_bp (Utilities|Casting|CastToPlayerStandinBP (Game|GetPlayerCharacter 0)))
  (Widget|SetVisibility (Variables|/Game/Blueprints/UI/HUD.HUD_C|GetInteractPrompt (Variables|/Game/Blueprints/PlayerStandinBP.PlayerStandinBP_C|GetHUDInstance _asplayer_standin_bp)) "SelfHitTestInvisible"))

(event Collision|EventActorEndOverlap
  (params (OtherActor :type Actor%20Object%20Reference))
  (Input|DisableInput (Game|GetPlayerController 0))
  (bind _asplayer_standin_bp (Utilities|Casting|CastToPlayerStandinBP (Game|GetPlayerCharacter 0)))
  (Widget|SetVisibility (Variables|/Game/Blueprints/UI/HUD.HUD_C|GetInteractPrompt (Variables|/Game/Blueprints/PlayerStandinBP.PlayerStandinBP_C|GetHUDInstance _asplayer_standin_bp)) "Hidden"))

(event Input|ActionEvents|InputActionInteract
  (params (Key :type Key%20Structure :default "None"))
  (:Pressed
    (if (not (Variables|Default|GetSeenBefore))
      (Variables|Default|SetSeenBefore true)
      (bind _asplayer_standin_bp (Utilities|Casting|CastToPlayerStandinBP (Game|GetPlayerCharacter 0)))
      (Variables|/Game/Blueprints/PlayerStandinBP.PlayerStandinBP_C|SetHasPaper _asplayer_standin_bp true)
      (Actor|DestroyActor))))

(fn ConstructionScript
  (Utilities|IsValid (Variables|VisualElements|GetClueMesh)
    (:Is%20Valid
      (Components|StaticMesh|SetStaticMesh (Variables|Default|GetCluePlaceholder) (Variables|VisualElements|GetClueMesh))
      (Components|Box|SetBoxExtent (Variables|Default|GetBox) (Variables|Collisions|GetCollisionSize) true))))