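; MoveBetweenAreas is an interactable area transition with two trigger boxes, Box and Box1.
; Overlap begin and end toggle the actor's input and the InteractPrompt on PlayerStandinBP's HUD.
; Pressing Interact inside either box starts a fade to black and immediately opens the EmmaPlayground level.
; Each branch stores the opposite box's location in Destination, which is never used, and the fade-in is unconnected.
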(event EventBeginPlay)

(event EventTick
  (params (DeltaSeconds :type Float%20%28single-precision%29)))

(event Collision|EventActorBeginOverlap
  (params (OtherActor :type Actor%20Object%20Reference))
  (Input|EnableInput (Game|GetPlayerController 0))
  (bind _asplayer_standin_bp (Utilities|Casting|CastToPlayerStandinBP (Game|GetPlayerCharacter 0)))
  (Widget|SetVisibility (Variables|/Game/Blueprints/UI/HUD.HUD_C|GetInteractPrompt (Variables|/Game/Blueprints/PlayerStandinBP.PlayerStandinBP_C|GetHUDInstance _asplayer_standin_bp)) "SelfHitTestInvisible"))

(event Collision|EventActorEndOverlap
  (params (OtherActor :type Actor%20Object%20Reference))
  (Input|DisableInput (Game|GetPlayerController 0))
  (bind _asplayer_standin_bp (Utilities|Casting|CastToPlayerStandinBP (Game|GetPlayerCharacter 0)))
  (Widget|SetVisibility (Variables|/Game/Blueprints/UI/HUD.HUD_C|GetInteractPrompt (Variables|/Game/Blueprints/PlayerStandinBP.PlayerStandinBP_C|GetHUDInstance _asplayer_standin_bp)) "Hidden"))

(event Input|ActionEvents|InputActionInteract
  (params (Key :type Key%20Structure :default "None"))
  (bind _returnvalue (Game|GetPlayerCharacter 0))
  (:Pressed
    (if (Collision|IsOverlappingActor (Variables|Default|GetBox1) _returnvalue :!class /Script/Engine.PrimitiveComponent)
      (Variables|Default|SetDestination (.location (Transformation|GetWorldTransform (Variables|Default|GetBox))))
      (CameraFades|StartCameraFade :self (Game|GetPlayerCameraManager 0) :ToAlpha 1.0 :Duration 2.0 :bShouldFadeAudio true :!label _label)
      (Game|OpenLevel(byObjectReference) "/Game/Levels/EmmaPlayground.EmmaPlayground")
      (elif (Collision|IsOverlappingActor (Variables|Default|GetBox) _returnvalue :!class /Script/Engine.PrimitiveComponent)
        (Variables|Default|SetDestination (Transformation|GetWorldLocation (Variables|Default|GetBox1)))
        (goto _label)))))

(fn ConstructionScript)