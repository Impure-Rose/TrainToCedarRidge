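; Interactable plunger mini-game actor where the player repeatedly presses E to fill a progress bar and reveal a clue.
; Overlap toggles input and the player HUD's interact prompt; the first E press opens a QTE widget.
; Later presses switch to the player's Camera1 and add progress toward Max.
; On completion the original camera returns and a PlungerFoundClue widget replaces the QTE, dismissed with another E press.
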(event Custom|BeginPlunging
  (Variables|Default|SetMiniGameActive true)
  (bind _returnvalue (UserInterface|CreateWidget "/Game/Blueprints/UI/QTE.QTE_C"))
  (UserInterface|Viewport|AddtoViewport _returnvalue 0)
  (bind _asplayer_standin_bp (Utilities|Casting|CastToPlayerStandinBP (Game|GetPlayerCharacter 0)))
  (Widget|SetVisibility (Variables|/Game/Blueprints/UI/HUD.HUD_C|GetInteractPrompt (Variables|/Game/Blueprints/PlayerStandinBP.PlayerStandinBP_C|GetHUDInstance _asplayer_standin_bp)) "Hidden"))

(event EventBeginPlay)

(event EventTick
  (params (DeltaSeconds :type Float%20%28single-precision%29)))

(event Collision|EventActorBeginOverlap
  (params (OtherActor :type Actor%20Object%20Reference))
  (Input|EnableInput (Game|GetPlayerController 0))
  (bind _asplayer_standin_bp (Utilities|Casting|CastToPlayerStandinBP (Game|GetPlayerCharacter 0)))
  (Widget|SetVisibility (Variables|/Game/Blueprints/UI/HUD.HUD_C|GetInteractPrompt (Variables|/Game/Blueprints/PlayerStandinBP.PlayerStandinBP_C|GetHUDInstance _asplayer_standin_bp)) "SelfHitTestInvisible"))

(event Collision|EventActorEndOverlap
  (params (OtherActor :type Actor%20Object%20Reference))
  (Input|DisableInput (Game|GetPlayerController 0))
  (bind _asplayer_standin_bp (Utilities|Casting|CastToPlayerStandinBP (Game|GetPlayerCharacter 0)))
  (Widget|SetVisibility (Variables|/Game/Blueprints/UI/HUD.HUD_C|GetInteractPrompt (Variables|/Game/Blueprints/PlayerStandinBP.PlayerStandinBP_C|GetHUDInstance _asplayer_standin_bp)) "Hidden"))

(event Input|KeyboardEvents|E
  (params (Key :type Key%20Structure :default "None"))
  (:Pressed
    (if (Variables|Default|GetMiniGameActive)
      (if (Variables|Default|Getwon)
        (Widget|RemovefromParent (Variables|Default|GetWinNotif))
        (else
          (bind _asplayer_standin_bp (Utilities|Casting|CastToPlayerStandinBP (Game|GetPlayerCharacter 0)))
          (Components|Activation|Activate (Variables|/Game/Blueprints/PlayerStandinBP.PlayerStandinBP_C|GetCamera1 _asplayer_standin_bp) false)
          (Components|Activation|Deactivate (Variables|/Game/Blueprints/PlayerStandinBP.PlayerStandinBP_C|GetCamera _asplayer_standin_bp))
          (bind _output_get (Variables|Default|SetCompletionLevel (+ (Variables|Default|GetCompletionLevel) (Variables|Default|Getplungemultiplier))))
          (Progress|SetPercent (Variables|/Game/Blueprints/UI/QTE.QTE_C|GetProgressBar_1 (stale Custom|BeginPlunging _returnvalue)) (/ _output_get (Variables|Default|Getmax)))
          (if (>= (Variables|Default|GetCompletionLevel) (Variables|Default|Getmax))
            (Development|PrintString "win")
            (Variables|Default|Setwon true)
            (bind _asplayer_standin_bp_2 (Utilities|Casting|CastToPlayerStandinBP (Game|GetPlayerCharacter 0)))
            (Components|Activation|Activate (Variables|/Game/Blueprints/PlayerStandinBP.PlayerStandinBP_C|GetCamera _asplayer_standin_bp_2) false)
            (Components|Activation|Deactivate (Variables|/Game/Blueprints/PlayerStandinBP.PlayerStandinBP_C|GetCamera1 _asplayer_standin_bp_2))
            (Widget|RemovefromParent (stale Custom|BeginPlunging _returnvalue))
            (bind _returnvalue (UserInterface|CreateWidget "/Game/Blueprints/UI/plungerFoundClue.plungerFoundClue_C" (Game|GetPlayerController 0)))
            (bind _output_get_2 (Variables|Default|SetWinNotif _returnvalue))
            (UserInterface|Viewport|AddtoViewport _returnvalue 0))))
      (else
        (CallFunction|BeginPlunging)))))

(fn ConstructionScript)